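; Football game state that keeps replicated scores for the Red and Blue teams.
; A RegisterGoal event passes the goal's team tag to RegisterScore, which credits the opposing team, so a Blue goal increments the Red score.
; Each score's RepNotify calls the OnScoreUpdated dispatcher with both current scores for any listeners.
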(event `/Game/Showcase/Blueprints/Interfaces/I_Football.Register Goal`
  (params (Goal :type "/Game/Showcase/Blueprints/Football/BP_Goal Object Reference") (Ball :type "/Game/Showcase/Blueprints/Football/BP_Ball Object Reference"))
  (`self.Register Score` (`/Game/Showcase/Blueprints/Football/BP_Goal.Goal Team` Goal)))

(fn `OnRep_Blue Team Score`
  (`self.On Score Updated` (make `ScoreboardData` (`self.Blue Team Score`) (`self.Red Team Score`))))

(fn `OnRep_Red Team Score`
  (`self.On Score Updated` (make `ScoreboardData` (`self.Blue Team Score`) (`self.Red Team Score`))))

(fn `Register Score`
  (params (Team :type "GameplayTag Structure"))
  (`|SwitchGameplayTag` Team
    (:`Football.Team.Blue`
      (bind _result (`/Engine/EditorBlueprintResources/StandardMacros.IncrementInt` (`self.Red Team Score`))
        (:`  `
          (set `self.Red Team Score` _result))))
    (:`Football.Team.Red`
      (bind _result_2 (`/Engine/EditorBlueprintResources/StandardMacros.IncrementInt` (`self.Blue Team Score`))
        (:`  `
          (set `self.Blue Team Score` _result_2))))))

(fn `UserConstructionScript`)