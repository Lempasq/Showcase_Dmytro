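; Game mode for a football match that runs match state, team assignment, ball spawning and goal celebrations.
; Match start spawns the ball and sorts teams, alternating Red and Blue gameplay tags by controller index; logins outside the lobby poll each tick for a pawn before sorting.
; Goals notify the game state and goal, pause the ball and focus player cameras on the goal for the celebration.
; The match-state RepNotify clears camera focus when play resumes.
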(event `self.K2_PostLogin`
  (params (NewPlayer :type "PlayerController Object Reference"))
  (if (`|EnumInequality` (`self.Current Match State`) "InLobby")
    (`/Engine/EditorBlueprintResources/StandardMacros.IsValid` (`Controller.K2_GetPawn` NewPlayer) :!label _label
      (:`Is Valid`
        (`self.Sort Teams`))
      (:`Is Not Valid`
        (`KismetSystemLibrary.DelayUntilNextTick`)
        (goto _label)))))

(event `Start The Match`
  (`/Engine/EditorBlueprintResources/StandardMacros.DoOnce` false
    (:`Completed`
      (set `self.Current Match State` "OnGoingMatch")
      (`self.Sort Teams`)
      (`self.Spawn The Ball`))))

(event `/Game/Showcase/Blueprints/Interfaces/I_Football.Register Goal`
  (params (Goal :type "/Game/Showcase/Blueprints/Football/BP_Goal Object Reference") (Ball :type "/Game/Showcase/Blueprints/Football/BP_Ball Object Reference"))
  (`/Game/Showcase/Blueprints/Football/BP_Ball.bIsActive` Ball
    (:`then`
      (set `self.Current Match State` "Celebrating")
      (message `/Game/Showcase/Blueprints/Interfaces/I_Football.Register Goal` (`GameplayStatics.GetGameState`) Goal Ball)
      (`self.Set Players Camera Focus` Goal)
      (`/Game/Showcase/Blueprints/Football/BP_Goal.On Goal Registered` Goal Ball (`self.Celebration Duration`))
      (set `/Game/Showcase/Blueprints/Football/BP_Ball.bIsActive` false Ball)
      (`KismetSystemLibrary.Delay` (`self.Celebration Duration`))
      (set `/Game/Showcase/Blueprints/Football/BP_Ball.bIsActive` true Ball)
      (set `self.Current Match State` "OnGoingMatch"))
    (:`else`)))

(fn `OnRep_Current Match State`
  (switch `EMatchStates` (`self.Current Match State`)
    (:`OnGoingMatch`
      (`self.Set Players Camera Focus` null))))

(fn `Set Players Camera Focus`
  (params (Actor :type "Actor Object Reference"))
  (bind _returnvalue (`GameplayStatics.GetNumPlayerControllers`))
  (if (> _returnvalue 0)
    (for _index (range (+ _returnvalue 1))
      (bind _returnvalue_2 (`GameplayStatics.GetPlayerController` _index))
      (`/Engine/EditorBlueprintResources/StandardMacros.IsValid` _returnvalue_2
        (:`Is Valid`
          (bind _asbp_player_controller_third_person (cast `/Game/Showcase/Blueprints/Characters/BP_PlayerController_ThirdPerson` _returnvalue_2))
          (set `/Game/Showcase/Blueprints/Characters/BP_PlayerController_ThirdPerson.Actor Camera Focus` Actor _asbp_player_controller_third_person))))))

(fn `Sort Teams`
  (bind _returnvalue (`GameplayStatics.GetNumPlayerControllers`))
  ; Sort teams after any player is ready
  (if (> _returnvalue 0)
    (for _index (range _returnvalue)
      (bind _returnvalue_2 (`GameplayStatics.GetPlayerController` _index))
      (`/Engine/EditorBlueprintResources/StandardMacros.IsValid` _returnvalue_2
        (:`Is Valid`
          (bind _returnvalue_3 (`Controller.K2_GetPawn` _returnvalue_2))
          (`/Engine/EditorBlueprintResources/StandardMacros.IsValid` _returnvalue_3
            (:`Is Valid`
              (bind _returnvalue_4 (message `ActorGameplayTagsInterface.HasGameplayTag` _returnvalue_3 (struct :`TagName` "Football.Team")))
              (if (not _returnvalue_4)
                (message `ActorGameplayTagsInterface.AddGameplayTag` _returnvalue_3 (select `bool` (`KismetMathLibrary.Conv_IntToBool` (mod _index 2)) :`false` (struct :`TagName` "Football.Team.Red") :`true` (struct :`TagName` "Football.Team.Blue") :!type "GameplayTag Structure"))))))))))

(fn `Spawn The Ball`
  (bind _output (`|ConvertAsset` (defaults `/Game/Showcase/Blueprints/Football/BP_Ball` "/Game/Showcase/Blueprints/Football/BP_Ball.BP_Ball_C")))
  (`/Engine/EditorBlueprintResources/StandardMacros.IsValid` _output
    (:`Is Valid`
      (bind _returnvalue (`|SpawnActorFromClass` "/Game/Showcase/Blueprints/Football/BP_Ball.BP_Ball_C" (`self.GetTransform` _output) "AlwaysSpawn" "MultiplyWithRoot" self null))
      (set `/Game/Showcase/Blueprints/Football/BP_Ball.bIsActive` true _returnvalue))))

(fn `UserConstructionScript`)