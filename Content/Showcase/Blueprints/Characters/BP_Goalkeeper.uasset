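; AI football goalkeeper that slides toward where the ball is heading to block it.
; Each Tick, it tracks a "Ball"-tagged component inside its scan volume, extrapolates its velocity half a second ahead, clamps that point to NavigableArea and interpolates the capsule there at ReactionSpeed.
; Without a ball in range, it targets its root position.
; Physical animation drives bones below a chosen bone, and construction tints the body by team gameplay tag.
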(event `self.ReceiveBeginPlay`
  (`parent.ReceiveBeginPlay`)
  (`self.Setup Physical Animation`))

(event `self.ReceiveTick`
  (params (DeltaSeconds :type "Float (single-precision)"))
  (bind _capsule (`self.Capsule`))
  ; Goal Keeper Logic : Finds the Predicted ball Location in T seconds and Smoothly moves to predicted Location
  (`parent.ReceiveTick` DeltaSeconds)
  (bind _predictedlocation (`self.Find Ball Predicted Location`))
  (bind _returnvalue (`KismetMathLibrary.VInterpTo` (`SceneComponent.K2_GetComponentLocation` (`self.Capsule`)) _predictedlocation (`GameplayStatics.GetWorldDeltaSeconds`) (`self.Reaction Speed`)))
  (if (!= (`SceneComponent.K2_GetComponentLocation` _capsule) _returnvalue :`ErrorTolerance` 0.1)
    (`SceneComponent.K2_SetWorldLocation` _capsule _returnvalue false false) ; Interp to predicted location
  ))

(fn `Assign Team Color`
  (bind _returnvalue (`PrimitiveComponent.CreateDynamicMaterialInstance` (`self.Mesh`) 0 "/Game/Showcase/Characters/BungeeMan/Materials/Mat_BungeeMan_Body.Mat_BungeeMan_Body" "None")) ; setup goal keeper team color
  (`|SwitchGameplayTagContainer` (`self.Team`)
    (:`Default`
      (`MaterialInstanceDynamic.SetVectorParameterValue` _returnvalue "TeamColor" (struct :`R` 1.0 :`G` 0.921582 :`B` 0.938686 :`A` 1.0)))
    (:`(GameplayTags=((TagName="Football.Team.Blue")))`
      (`MaterialInstanceDynamic.SetVectorParameterValue` _returnvalue "TeamColor" (struct :`G` 0.14996 :`B` 1.0 :`A` 1.0)))
    (:`(GameplayTags=((TagName="Football.Team.Red")))`
      (`MaterialInstanceDynamic.SetVectorParameterValue` _returnvalue "TeamColor" (struct :`R` 1.0 :`G` 0.074214 :`A` 1.0)))))

(fn `Find Ball Predicted Location`
  (returns (PredictedLocation :type "Vector Structure"))
  (bind _ball_scan_collision (`self.Ball Scan Collision`))
  (bind _target_ball (`self.Target Ball`)
    (:`then`
      (if (`PrimitiveComponent.IsOverlappingComponent` _target_ball _ball_scan_collision)
        (return (`PrimitiveComponent.GetClosestPointOnCollision` (`self.NavigableArea`) (`self.Predict Location At Time` _target_ball 0.5) "None"))
        (else
          (set `self.Target Ball` null))))
    (:`else`
      (for _array_element (`PrimitiveComponent.GetOverlappingComponents` _ball_scan_collision)
        (if (`ActorComponent.ComponentHasTag` _array_element "Ball")
          (set `self.Target Ball` _array_element)
          (return (`SceneComponent.K2_GetComponentLocation` (`self.DefaultSceneRoot`)))))))
  (return (`SceneComponent.K2_GetComponentLocation` (`self.DefaultSceneRoot`))))

(fn `Predict Location At Time`
  (params (PhysicComponent :type "PrimitiveComponent Object Reference") (PredictionTime :type "Float (double-precision)"))
  (returns (PredictedLocation :type "Vector Structure"))
  ; Predict the future ball position in T seconds based on current velocity
  (bind _returnvalue (`PrimitiveComponent.GetPhysicsLinearVelocity` PhysicComponent "None"))
  (return (+ (`SceneComponent.K2_GetComponentLocation` PhysicComponent) (* _returnvalue PredictionTime))))

(fn `Setup Physical Animation`
  (bind _mesh (`self.Mesh`))
  (bind _physica_lanim_bone (`self.Physica lAnim Bone`))
  (`PhysicalAnimationComponent.SetSkeletalMeshComponent` (`self.PhysicalAnimation`) _mesh)
  (`SkeletalMeshComponent.SetAllBodiesBelowSimulatePhysics` _mesh _physica_lanim_bone true false)
  (`PhysicalAnimationComponent.ApplyPhysicalAnimationSettingsBelow` (`self.PhysicalAnimation`) _physica_lanim_bone (make `PhysicalAnimationData` true 5000.0 500.0 5000.0 500.0) false))

(fn `UserConstructionScript`
  (`self.Assign Team Color`))