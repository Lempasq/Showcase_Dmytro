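; BP_Ball is the football actor for a team football game, tracking its current dribbler and showing that player's team color.
; The bIsActive RepNotify toggles physics and visibility; on authority it also clears the dribbler and, when active, teleports the ball to its default position.
; The CurrentDribbler RepNotify shows the trail and tints it and a dynamic decal material blue, red or default white from the dribbler's gameplay tags.
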(event `self.ReceiveBeginPlay`
  (`parent.ReceiveBeginPlay`)
  (bind _returnvalue (`DecalComponent.CreateDynamicMaterialInstance` (`self.Decal`)))
  (set `self.Ball Decal Mat` _returnvalue))

(event `/Game/Showcase/Blueprints/Interfaces/I_Ball.Set Dribbler`
  (params (`New Dribbler` :type "Actor Object Reference"))
  (set `self.Current Dribbler` `New Dribbler`))

(fn `OnRep_bIsActive`
  (bind _bisactive (`self.bIsActive`))
  (bind (_returnvalue_location _returnvalue_rotation) (`KismetMathLibrary.BreakTransform` (`self.GetTransform` (`|ConvertAsset` (`self.Default Position`)))))
  (`PrimitiveComponent.SetSimulatePhysics` (`self.StaticMeshComponent`) _bisactive)
  (`self.SetActorHiddenInGame` (not _bisactive))
  (`/Engine/EditorBlueprintResources/ActorMacros.Switch Has Authority`
    (:`Authority`
      (set `self.Current Dribbler` null)
      (if (`self.bIsActive`)
        (`self.K2_SetActorLocationAndRotation` _returnvalue_location _returnvalue_rotation false true)))))

(fn `OnRep_Current Dribbler`
  (bind _ball_decal_mat (`self.Ball Decal Mat`))
  (bind _trail (`self.Trail`))
  (`SceneComponent.SetVisibility` (`self.Trail`) (`KismetSystemLibrary.IsValid` (`self.Current Dribbler`)) false)
  (bind _current_dribbler (`self.Current Dribbler`)
    (:`then`
      (bind _returnvalue (message `ActorGameplayTagsInterface.GetGameplayTagContainer` _current_dribbler))
      (`|SwitchGameplayTagContainer` _returnvalue
        (:`Default`
          (`FXSystemComponent.SetColorParameter` _trail "TeamColor" (struct :`R` 1.0 :`G` 1.0 :`B` 1.0 :`A` 1.0) :!label _label)
          (`MaterialInstanceDynamic.SetVectorParameterValue` _ball_decal_mat "TeamColor" (struct :`R` 1.0 :`G` 1.0 :`B` 1.0 :`A` 1.0)))
        (:`(GameplayTags=((TagName="Football.Team.Blue")))`
          (`FXSystemComponent.SetColorParameter` _trail "TeamColor" (struct :`G` 0.174647 :`B` 1.0 :`A` 1.0))
          (`MaterialInstanceDynamic.SetVectorParameterValue` _ball_decal_mat "TeamColor" (struct :`G` 0.174647 :`B` 1.0 :`A` 1.0)))
        (:`(GameplayTags=((TagName="Football.Team.Red")))`
          (`FXSystemComponent.SetColorParameter` _trail "TeamColor" (struct :`R` 1.0 :`B` 0.026241 :`A` 1.0))
          (`MaterialInstanceDynamic.SetVectorParameterValue` _ball_decal_mat "TeamColor" (struct :`R` 1.0 :`B` 0.026241 :`A` 1.0)))))
    (:`else`
      (goto _label))))

(fn `UserConstructionScript`)