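; Team-assigned goal for the football showcase that detects balls and plays a celebration when a goal is registered.
; On authority, ball overlaps are reported to the GameMode; OnGoalRegistered sets Celebrating for a retriggerable duration and spawns a Niagara hit effect tinted by GoalTeam.
; OnRep_bCelebrating swaps the net to RandColor during celebration, then restores the team materials that the construction script applies from the GoalTeam gameplay tag.
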(event `self.Goal Collision.OnComponentBeginOverlap`
  (params (OverlappedComponent :type "PrimitiveComponent Object Reference") (OtherActor :type "Actor Object Reference") (OtherComp :type "PrimitiveComponent Object Reference") (OtherBodyIndex :type Integer) (bFromSweep :type Boolean) (SweepResult :type "HitResult Structure (by ref)"))
  (`/Engine/EditorBlueprintResources/ActorMacros.Switch Has Authority`
    (:`Authority`
      (bind _asbp_ball (cast `/Game/Showcase/Blueprints/Football/BP_Ball` OtherActor))
      (message `/Game/Showcase/Blueprints/Interfaces/I_Football.Register Goal` (`GameplayStatics.GetGameMode`) self _asbp_ball))))

(event `On Goal Registered`
  (params (Ball :type "/Game/Showcase/Blueprints/Football/BP_Ball Object Reference") (`Celebration Duration` :type "Float (single-precision)"))
  (bind (_returnvalue_location _returnvalue_rotation) (`KismetMathLibrary.BreakTransform` (`self.GetTransform` Ball)))
  (`|ExecutionSequence`
    (:`then_0`
      (`/Engine/EditorBlueprintResources/ActorMacros.Switch Has Authority`
        (:`Authority`
          (set `self.bCelebrating` true)
          (`KismetSystemLibrary.RetriggerableDelay` `Celebration Duration`)
          (set `self.bCelebrating` false))))
    (:`then_1`
      (bind _returnvalue (`NiagaraFunctionLibrary.SpawnSystemAtLocation` "/Game/Showcase/VFX/BasicHit/NS_BasicHit.NS_BasicHit" _returnvalue_location _returnvalue_rotation))
      (`/Engine/EditorBlueprintResources/StandardMacros.IsValid` _returnvalue
        (:`Is Valid`
          (`|SwitchGameplayTag` (`self.Goal Team`)
            (:`Football.Team.Blue`
              (`FXSystemComponent.SetColorParameter` _returnvalue "TeamColor" (struct :`R` 1.0 :`G` 0.502887 :`B` 0.502887 :`A` 1.0)))
            (:`Football.Team.Red`
              (`FXSystemComponent.SetColorParameter` _returnvalue "TeamColor" (struct :`R` 0.502887 :`G` 0.502887 :`B` 1.0 :`A` 1.0)))))))))

(fn `Assign Team Color`
  (bind _goal_mesh (`self.Goal Mesh`))
  (bind _goal_line (`self.Goal Line`))
  (bind _goal_mesh_2 (`self.Goal Mesh`))
  (`|SwitchGameplayTag` (`self.Goal Team`)
    (:`Football.Team.Blue`
      (`PrimitiveComponent.SetMaterial` _goal_mesh_2 0 "/Game/Showcase/Materials/BlueSimple.BlueSimple")
      (`PrimitiveComponent.SetMaterial` _goal_mesh 1 "/Game/Showcase/Materials/BlueNet.BlueNet")
      (`PrimitiveComponent.SetMaterial` _goal_line 0 "/Game/Showcase/Materials/BlueGoalLine.BlueGoalLine"))
    (:`Football.Team.Red`
      (`PrimitiveComponent.SetMaterial` _goal_mesh_2 0 "/Game/Showcase/Materials/RedSimple.RedSimple")
      (`PrimitiveComponent.SetMaterial` _goal_mesh 1 "/Game/Showcase/Materials/RedNet.RedNet")
      (`PrimitiveComponent.SetMaterial` _goal_line 0 "/Game/Showcase/Materials/RedGoalLine.RedGoalLine"))))

(fn `OnRep_bCelebrating`
  (if (`self.bCelebrating`)
    (`PrimitiveComponent.SetMaterial` (`self.Goal Mesh`) 1 "/Game/Showcase/Materials/RandColor.RandColor")
    (else
      (`self.Assign Team Color`))))

(fn `OnRep_IsGoalActive`
  (if (`self.bCelebrating`)
    (`self.Assign Team Color`)
    (else
      (`PrimitiveComponent.SetMaterial` (`self.Goal Mesh`) 1 "/Game/Showcase/Materials/RandColor.RandColor"))))

(fn `UserConstructionScript`
  (`self.Assign Team Color`))